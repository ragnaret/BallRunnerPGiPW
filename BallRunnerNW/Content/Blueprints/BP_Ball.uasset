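; Player-controlled rolling ball that fades in from full fade at BeginPlay and reloads the current level when it takes any damage.
; Forward/back and left/right axis inputs apply acceleration-based torque to the Sphere, scaled by ForceMultiply.
; ChangeCameraView sets spring arm length and world pitch and yaw.
; RestartLevel offers a once-only fade-out before reopening the level, while the damage event reopens it immediately.
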(event `self.ReceiveBeginPlay`
  (`PlayerCameraManager.StartCameraFade` :`self` (`GameplayStatics.GetPlayerCameraManager` 0) :`FromAlpha` 1.0 :`Duration` 3.0))

(event `InputAxis|ForwardBack`
  (params (AxisValue :type "Float (single-precision)"))
  ;[1 1 1] Ball Movement in Torque
  (`PrimitiveComponent.AddTorqueInRadians` (`self.Sphere`) (`KismetMathLibrary.MakeVector` 0.0 (* AxisValue (`self.ForceMultiply`))) "None" true))

(event `InputAxis|LeftRight`
  (params (AxisValue :type "Float (single-precision)"))
  ;[1 1 1] Ball Movement in Torque
  (`PrimitiveComponent.AddTorqueInRadians` (`self.Sphere`) (`KismetMathLibrary.MakeVector` (* AxisValue (`self.ForceMultiply`))) "None" true))

(event `self.ReceiveAnyDamage`
  (params (Damage :type "Float (single-precision)") (DamageType :type "DamageType Object Reference") (InstigatedBy :type "Controller Object Reference") (DamageCauser :type "Actor Object Reference"))
  (bind _returnvalue (`GameplayStatics.GetCurrentLevelName` true))
  (`GameplayStatics.OpenLevel` (`KismetStringLibrary.Conv_StringToName` _returnvalue)))

(fn `ChangeCameraView`
  (params (`Camera Position` :type "Float (double-precision)") (`Camera Rotation Y` :type "Float (double-precision)") (`Camera Rotation Z` :type "Float (double-precision)"))
  (bind _springarm (`self.SpringArm`))
  (set `SpringArmComponent.TargetArmLength` `Camera Position` _springarm)
  (`SceneComponent.K2_SetWorldRotation` _springarm (`KismetMathLibrary.MakeRotator` 0.0 `Camera Rotation Y` `Camera Rotation Z`) false false))

(fn `UserConstructionScript`)